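; BP_player is the player Character, with walking, camera look, jumping, sprinting and a toggleable spotlight.
; Axis inputs drive movement along the actor's forward and right vectors and feed controller yaw and pitch.
; Holding sprint doubles the max walk speed until release, and the F key, bound directly, toggles SpotLight visibility.
; SanityDrain is an unfinished stub with unconnected clamp, subtract and print nodes.
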(event `InputAction|sprint`
  (params (Key :type "Key Structure"))
  (bind _charactermovement (`self.CharacterMovement`))
  ;[1 1 1] sprint/jump
  (:`Pressed`
    (set `CharacterMovementComponent.MaxWalkSpeed` 900.0 _charactermovement))
  (:`Released`
    (set `CharacterMovementComponent.MaxWalkSpeed` 450.0 _charactermovement)))

(event `InputAxis|forward/back`
  (params (AxisValue :type "Float (single-precision)"))
  ;[1 1 1] player movement
  (`self.AddMovementInput` (`self.GetActorForwardVector`) AxisValue))

(event `InputAxis|camera yaw`
  (params (AxisValue :type "Float (single-precision)"))
  ;[1 1 1] camera movement
  (`self.AddControllerYawInput` AxisValue))

(event `InputAction|jump`
  (params (Key :type "Key Structure"))
  ;[1 1 1] sprint/jump
  (:`Pressed`
    (`self.Jump`)))

(event `InputAxis|camera pitch`
  (params (AxisValue :type "Float (single-precision)"))
  ;[1 1 1] camera movement
  (`self.AddControllerPitchInput` AxisValue))

(event `InputAxis|MoveRight`
  (params (AxisValue :type "Float (single-precision)"))
  ;[1 1 1] player movement
  (`self.AddMovementInput` (`self.GetActorRightVector`) AxisValue))

(event `Key|F`
  (params (Key :type "Key Structure"))
  (:`Pressed`
    (`SceneComponent.ToggleVisibility` (`self.SpotLight`) false)))

(fn `sanityDrain`)

(fn `UserConstructionScript`)